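; BPC_DialogueComponent is a component that runs line-by-line dialogue from a dialogue asset.
; StartDialogue stores the asset, resets the line index and broadcasts OnDialogueStarted with the first line.
; AdvanceDialogue re-broadcasts that same dispatcher for each following line, then fires OnDialogueEnded and clears the state after the last one.
; CancelDialogue clears the active dialogue immediately and fires OnDialogueEnded.
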(fn StartDialogue
  (params (Dialogue :type DA%20Dialogue%20Object%20Reference))
  (Variables|Default|SetCurrentDialogue Dialogue)
  (Variables|Default|SetCurrentLineIndex 0)
  (Variables|Default|SetIsDialogueActive true)
  (Utilities|IsValid Dialogue
    (:Is%20Valid
      (Default|CallOnDialogueStarted (Utilities|Array|Get(acopy) (Variables|/Game/Nutbound/DA_Dialogue.DA_Dialogue_C|GetLines Dialogue))))))

(fn AdvanceDialogue
  (bind _currentlineindex (Variables|Default|GetCurrentLineIndex))
  (if (Variables|Default|GetIsDialogueActive)
    (Math|Integer|IncrementInt _currentlineindex
      (:%20%20
        (if (< _currentlineindex (Utilities|Array|Length (Variables|/Game/Nutbound/DA_Dialogue.DA_Dialogue_C|GetLines (Variables|Default|GetCurrentDialogue))))
          (Default|CallOnDialogueStarted (Utilities|Array|Get(acopy) (Variables|/Game/Nutbound/DA_Dialogue.DA_Dialogue_C|GetLines (Variables|Default|GetCurrentDialogue)) (Variables|Default|GetCurrentLineIndex)))
          (else
            (Variables|Default|SetIsDialogueActive false)
            (Default|CallOnDialogueEnded)
            (Variables|Default|SetCurrentDialogue 0)))))))

(fn CancelDialogue
  (Variables|Default|SetIsDialogueActive false)
  (Variables|Default|SetCurrentDialogue 0)
  (Default|CallOnDialogueEnded))