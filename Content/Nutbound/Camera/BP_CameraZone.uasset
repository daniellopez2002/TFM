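; BP_CameraZone is a trigger volume that switches the player's camera zone when the nut character enters it.
; On BeginPlay it caches the CameraController from the possessed BP_NutCharacter.
; When that character overlaps the collision mesh, it sets an activated flag and passes itself to ChangeCameraZone, so it fires once unless the flag is cleared elsewhere.
; A debug print of the zone's camera state is left unconnected.
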(event OnComponentBeginOverlap(CollisionMesh)
  (params (OverlappedComponent :type Primitive%20Component%20Object%20Reference) (OtherActor :type Actor%20Object%20Reference) (OtherComp :type Primitive%20Component%20Object%20Reference) (OtherBodyIndex :type Integer) (bFromSweep :type Boolean) (SweepResult :type Hit%20Result%20Structure%20%28by%20ref%29))
  (Class|KismetSystemLibrary|IsObjectOfSoftClass OtherActor "/Game/Nutbound/Blueprints/BP_NutCharacter.BP_NutCharacter_C"
    (:True
      (if (not (Variables|Default|GetIsBeenActivated))
        (Variables|Default|SetIsBeenActivated true)
        (Default|ChangeCameraZone (Variables|Default|GetCameraController) self)))))

(event EventBeginPlay
  (bind _asbp_nut_character (Utilities|Casting|CastToBP_NutCharacter (Pawn|GetControlledPawn (Game|GetPlayerController 0))))
  (Variables|Default|SetCameraController (Variables|/Game/Nutbound/Blueprints/BP_NutCharacter.BP_NutCharacter_C|GetCameraController _asbp_nut_character)))

(event Collision|EventActorBeginOverlap
  (params (OtherActor :type Actor%20Object%20Reference)))

(event EventTick
  (params (DeltaSeconds :type Float%20%28single-precision%29)))

(fn ConstructionScript)