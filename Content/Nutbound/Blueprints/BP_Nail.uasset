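; BP_Nail is a short-lived projectile that launches itself at the player character on spawn.
; BeginPlay aims at the player's location with a small random offset, adds an upward bias for an arc, and sets the ProjectileMovement velocity.
; A box collision hit ends its flying state, damaging the player's Health component and destroying the nail if the player is struck first.
; Hitting another nail also destroys it.
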(event OnComponentHit(BoxCollision)
  (params (HitComponent :type Primitive%20Component%20Object%20Reference) (OtherActor :type Actor%20Object%20Reference) (OtherComp :type Primitive%20Component%20Object%20Reference) (NormalImpulse :type Vector :default "0, 0, 0") (Hit :type Hit%20Result%20Structure%20%28by%20ref%29))
  (bind _main_character (Variables|Default|GetMain%20Character))
  (Utilities|Casting|CastToBP_Nail OtherActor
    (:then
      (Actor|DestroyActor))
    (:CastFailed
      (if (Variables|Default|GetIsFlying)
        (Variables|Default|SetIsFlying false)
        (if (== OtherActor _main_character)
          (Default|TakeDamage (Variables|/Game/Nutbound/Blueprints/BP_NutCharacter.BP_NutCharacter_C|GetHealth _main_character) 1 (Transformation|GetActorLocation))
          (Actor|DestroyActor))))))

(event EventBeginPlay
  (bind _returnvalue (Game|GetPlayerCharacter 0))
  (bind _projectilemovement (Variables|Default|GetProjectileMovement))
  (Components|Movement|SetUpdatedComponent (Variables|Default|GetProjectileMovement) (Variables|Default|GetBoxCollision))
  (Variables|Default|SetIsFlying true)
  (Actor|SetLifeSpan 5.0)
  (bind _asbp_nut_character (Utilities|Casting|CastToBP_NutCharacter _returnvalue))
  (Variables|Default|SetMain%20Character _asbp_nut_character)
  (bind _output_get (Variables|Default|SetPlayerPosition (Transformation|GetActorLocation _returnvalue)))
  (bind _output_get_2 (Variables|Default|SetrandomOffset (* (Math|Random|RandomUnitVector) 2e+01)))
  (bind _output_get_3 (Variables|Default|SetTargetPoint (+ _output_get_2 _output_get)))
  (bind _output_get_4 (Variables|Default|SetDirection (Math|Vector|Normalize (- _output_get_3 (Transformation|GetActorLocation)))))
  (Variables|Default|SetDirection (Math|Vector|MakeVector (.x _output_get_4) (.y _output_get_4) (+ (.z _output_get_4) 0.3)))
  (Variables|Default|SetNormalizedDirection (Math|Vector|Normalize (Variables|Default|GetDirection)))
  (Variables|/Script/Engine.MovementComponent|SetVelocity _projectilemovement (* (Variables|Default|GetNormalizedDirection) 5e+02))
  (Development|PrintString (Utilities|String|ToString(Vector) (Variables|/Script/Engine.MovementComponent|GetVelocity _projectilemovement))))

(event Collision|EventActorBeginOverlap
  (params (OtherActor :type Actor%20Object%20Reference)))

(fn ConstructionScript)