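; BP_MainCharacter is the main player character in Nutbound, handling input setup, fall tracking and death.
; On BeginPlay it adds an Enhanced Input mapping context and runs PlayerDefaults, which enables input, turns off mesh physics and collision, and caches the HUD.
; Tick times continuous falling to set IsFallingVoid past a threshold, with debug printing.
; Health's OnDeath disables input and ragdolls the mesh; the move input and post-death delay lead nowhere.
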(event OnDeath(Health)
  (bind _mesh (Variables|Character|GetMesh))
  (Input|DisableInput (Game|GetPlayerController 0))
  (Collision|SetCollisionEnabled _mesh "QueryAndPhysics")
  (Physics|SetSimulatePhysics _mesh true)
  (Utilities|FlowControl|Delay 2.0))

(event Input|EnhancedActionEvents|EnhancedInputActionIA_Move
  (params (ActionValue :type Vector%202D%20Structure) (ElapsedSeconds :type Float%20%28double-precision%29) (TriggeredSeconds :type Float%20%28double-precision%29) (InputAction :type Input%20Action%20Object%20Reference :default "/Game/ThirdPerson/Input/Actions/IA_Move.IA_Move")))

(event EventBeginPlay
  (bind _asbp_player_controller (Utilities|Casting|CastToBP_PlayerController (Game|GetPlayerController 0)))
  (Utilities|IsValid (PlayerController|LocalPlayerSubsystems|GetEnhancedInputLocalPlayerSubsystem _asbp_player_controller)
    (:Is%20Valid
      (Input|AddMappingContext (PlayerController|LocalPlayerSubsystems|GetEnhancedInputLocalPlayerSubsystem _asbp_player_controller) 0 0 "(bIgnoreAllPressedKeysUntilRelease=True,bForceImmediately=False,bNotifyUserSettings=False)")
      (CallFunction|PlayerDefaults))))

(event Collision|EventActorBeginOverlap
  (params (OtherActor :type Actor%20Object%20Reference)))

(event EventTick
  (params (DeltaSeconds :type Float%20%28single-precision%29))
  (if (AI|Components|NavMovement|IsFalling (Variables|Character|GetCharacterMovement))
    (bind _output_get (Variables|Default|SetFallingCounter (+ (Variables|Default|GetFallingCounter) DeltaSeconds)))
    (Variables|Default|SetIsFallingVoid (>= _output_get (Variables|Default|GetMaxFallingTimer)))
    (Development|PrintString (Utilities|String|ToString(Float) (Variables|Default|GetFallingCounter)))
    (else
      (Variables|Default|SetFallingCounter 0.0)
      (Variables|Default|SetIsFallingVoid false))))

(fn ConstructionScript)

(fn PlayerDefaults
  (bind _mesh (Variables|Character|GetMesh))
  (Utilities|FlowControl|Sequence
    (:then_0
      (Input|EnableInput (Game|GetPlayerController 0))
      (Physics|SetSimulatePhysics _mesh false)
      (Collision|SetCollisionEnabled _mesh "NoCollision"))
    (:then_1
      (bind _returnvalue (Actor|GetActorOfClass "/Game/Nutbound/HUD/HUDClass.HUDClass_C"))
      (Variables|Default|SetHUD _returnvalue))))