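; BP_OilTrap is an oil trap hazard that, as wired, acts as a height-based kill plane for the player.
; BeginPlay caches player 0 as BP_NutCharacter, and Tick calls Respawn on it whenever its Z is at or below KillZ.
; The Box overlap event is empty; the contact-triggered delayed respawn and the Health damage calls are disconnected and never run.
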(event OnComponentBeginOverlap(Box)
  (params (OverlappedComponent :type Primitive%20Component%20Object%20Reference) (OtherActor :type Actor%20Object%20Reference) (OtherComp :type Primitive%20Component%20Object%20Reference) (OtherBodyIndex :type Integer) (bFromSweep :type Boolean) (SweepResult :type Hit%20Result%20Structure%20%28by%20ref%29)))

(event EventBeginPlay
  (bind _asbp_nut_character (Utilities|Casting|CastToBP_NutCharacter (Game|GetPlayerCharacter 0)))
  (Variables|Default|SetMain%20Character _asbp_nut_character))

(event EventTick
  (params (DeltaSeconds :type Float%20%28single-precision%29))
  (if (<= (.z (Transformation|GetActorLocation (Variables|Default|GetMain%20Character))) (Variables|Default|GetKillZ))
    (Class|NutCharacter|Respawn (Variables|Default|GetMain%20Character))))

(fn ConstructionScript)