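; Player nut character: handles hammer hits scaled by combo index, coin pickup into inventory, and enemy focus through an overlap sphere.
; Tick projects a fading ground shadow, flags long falls, updates focus, and builds energy while moving, driving VFX scale and light intensity.
; Attacking and jumping also add energy.
; Damage triggers knockback and a material flash timeline that toggles invulnerability; death explodes the nut and restarts the demo level via the GameInstance.
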(event OnDeath(Health)
  (Effects|SpawnEmitteratLocation "/Game/InfinityBladeEffects/Effects/FX_Cines/cinema03/P_CIN_IB_Explosion.P_CIN_IB_Explosion" (Transformation|GetActorLocation))
  (Rendering|SetVisibility (Variables|Character|GetMesh) false true)
  (Class|NutCharacter|Respawn))

(event OnComponentBeginOverlap(SphereFocus)
  (params (OverlappedComponent :type Primitive%20Component%20Object%20Reference) (OtherActor :type Actor%20Object%20Reference) (OtherComp :type Primitive%20Component%20Object%20Reference) (OtherBodyIndex :type Integer) (bFromSweep :type Boolean) (SweepResult :type Hit%20Result%20Structure%20%28by%20ref%29))
  (if (< (- (.z (Transformation|GetActorLocation)) (.z (Transformation|GetActorLocation OtherActor))) 2e+01)
    (if (and (Utilities|IsValid (Actor|GetComponentbyClass OtherActor "/Game/Nutbound/Components/Focusable.Focusable_C")) (not (Utilities|Array|ContainsItem (Variables|Default|GetActorsFocus) OtherActor)))
      (Utilities|Array|Add (Variables|Default|GetActorsFocus) OtherActor))))

(event OnComponentEndOverlap(SphereFocus)
  (params (OverlappedComponent :type Primitive%20Component%20Object%20Reference) (OtherActor :type Actor%20Object%20Reference) (OtherComp :type Primitive%20Component%20Object%20Reference) (OtherBodyIndex :type Integer))
  (if (Utilities|Array|ContainsItem (Variables|Default|GetActorsFocus) OtherActor)
    (Class|NutCharacter|RemoveActorfromFocus OtherActor)
    (Utilities|IsValid (Variables|Default|GetFocusCompnent)
      (:Is%20Valid
        (Variables|/Game/Nutbound/Components/Focusable.Focusable_C|SetIsFocused (Variables|Default|GetFocusCompnent) false)
        (Variables|Default|SetFocusCompnent 0)))))

(event OnComponentBeginOverlap(HammerCollision)
  (params (OverlappedComponent :type Primitive%20Component%20Object%20Reference) (OtherActor :type Actor%20Object%20Reference) (OtherComp :type Primitive%20Component%20Object%20Reference) (OtherBodyIndex :type Integer) (bFromSweep :type Boolean) (SweepResult :type Hit%20Result%20Structure%20%28by%20ref%29))
  (bind _comboindex (Variables|Default|GetComboIndex))
  (bind _returnvalue (* _comboindex 10))
  (if (Variables|Default|GetIsAttacking)
    (bind _astfmenemy (Utilities|Casting|CastToTFMEnemy OtherActor)
      (:then
        (Default|TakeDamage (Actor|GetComponentbyClass _astfmenemy "/Game/Nutbound/Components/Health.Health_C") _returnvalue (Transformation|GetActorLocation)))
      (:CastFailed
        (bind _asbp_grabber (Utilities|Casting|CastToBP_Grabber OtherActor))
        (Default|TakeDamage (Actor|GetComponentbyClass _asbp_grabber "/Game/Nutbound/Components/Health.Health_C") _returnvalue (Transformation|GetActorLocation))))))

(event OnComponentBeginOverlap(CapsuleComponent)
  (params (OverlappedComponent :type Primitive%20Component%20Object%20Reference) (OtherActor :type Actor%20Object%20Reference) (OtherComp :type Primitive%20Component%20Object%20Reference) (OtherBodyIndex :type Integer) (bFromSweep :type Boolean) (SweepResult :type Hit%20Result%20Structure%20%28by%20ref%29))
  (bind _asbp_nut_coin (Utilities|Casting|CastToBP_NutCoin OtherActor))
  (bind _success (Default|AddtoInventory (Variables|Default|GetAbilityInventory) "NutCoin" 1))
  (if _success
    (Default|PickUp _asbp_nut_coin)))

(event OnTakeDamage(Health)
  (params (AttackDirection :type Vector :default "0, 0, 0"))
  (Audio|PlaySoundatLocation (.OutItem (Utilities|Array|Random (Variables|Default|GetHitSound))) (Transformation|GetActorLocation) "0, 0, 0" 1.0 1.0 0.0 0 0 0 0)
  (Effects|SpawnEmitteratLocation "/Game/Realistic_Starter_VFX_Pack_Vol2/Particles/Destruction/P_Destruction_Metal.P_Destruction_Metal" (Transformation|GetActorLocation) "0, 0, 0" "1.000000,1.000000,1.000000" true "AutoRelease")
  (Character|LaunchCharacter (* AttackDirection 2e+01) false false)
  (CallFunction|ColorChange))

(event Custom|ColorChange
  (bind _color (Timeline|DamageColorEffect PlayFromStart)
    (:Update
      (Variables|Default|SetIsInvulnerable true)
      (for _array_element (Variables|Default|GetDynamicMaterials)
        (Rendering|Material|SetScalarParameterValue _array_element "DamageAmount" _color :!class /Script/Engine.MaterialInstanceDynamic)))
    (:Finished
      (for _array_element_2 (Variables|Default|GetDynamicMaterials)
        (Rendering|Material|SetScalarParameterValue _array_element_2 "DamageAmount" 0.0 :!class /Script/Engine.MaterialInstanceDynamic))
      (Variables|Default|SetIsInvulnerable false))))

(event Input|EnhancedActionEvents|EnhancedInputActionIA_Attack
  (params (ActionValue :type Boolean) (ElapsedSeconds :type Float%20%28double-precision%29) (TriggeredSeconds :type Float%20%28double-precision%29) (InputAction :type Input%20Action%20Object%20Reference :default "/Game/ThirdPerson/Input/Actions/IA_Attack.IA_Attack"))
  (Default|PlayerGainEnergy (Variables|Default|GetHealth) (Math|Conversions|ToFloat(Integer) (* (Variables|Default|GetComboIndex) 5))))

(event Input|EnhancedActionEvents|EnhancedInputActionIA_Dodge
  (params (ActionValue :type Boolean) (ElapsedSeconds :type Float%20%28double-precision%29) (TriggeredSeconds :type Float%20%28double-precision%29) (InputAction :type Input%20Action%20Object%20Reference :default "/Game/ThirdPerson/Input/Actions/IA_Dodge.IA_Dodge")))

(event Input|EnhancedActionEvents|EnhancedInputActionIA_Interact
  (params (ActionValue :type Boolean) (ElapsedSeconds :type Float%20%28double-precision%29) (TriggeredSeconds :type Float%20%28double-precision%29) (InputAction :type Input%20Action%20Object%20Reference :default "/Game/ThirdPerson/Input/Actions/IA_Interact.IA_Interact"))
  (:Started
    (Development|PrintString "Interact Placeholder")))

(event Input|EnhancedActionEvents|EnhancedInputActionIA_Jump
  (params (ActionValue :type Boolean) (ElapsedSeconds :type Float%20%28double-precision%29) (TriggeredSeconds :type Float%20%28double-precision%29) (InputAction :type Input%20Action%20Object%20Reference :default "/Game/ThirdPerson/Input/Actions/IA_Jump.IA_Jump"))
  (Default|PlayerGainEnergy (Variables|Default|GetHealth) 1e+01))

(event EventBeginPlay
  (for _index (range 0 (Rendering|Material|GetNumMaterials (Variables|Character|GetMesh)))
    (bind _returnvalue (Rendering|Material|CreateDynamicMaterialInstance (Variables|Character|GetMesh) _index "/Game/Nutbound/Models/Termuk/Materials/M_Nut.M_Nut" "None" :!class /Script/Engine.PrimitiveComponent))
    (Utilities|Array|Add (Variables|Default|GetDynamicMaterials) _returnvalue))
  (bind _asbp_player_controller (Utilities|Casting|CastToBP_PlayerController (Game|GetPlayerController 0)))
  (Utilities|IsValid (PlayerController|LocalPlayerSubsystems|GetEnhancedInputLocalPlayerSubsystem _asbp_player_controller)
    (:Is%20Valid
      (Input|AddMappingContext (PlayerController|LocalPlayerSubsystems|GetEnhancedInputLocalPlayerSubsystem _asbp_player_controller) "/Game/ThirdPerson/Input/IMC_Default.IMC_Default" 0 "(bIgnoreAllPressedKeysUntilRelease=True,bForceImmediately=False,bNotifyUserSettings=False)"))))

(event EventRespawn
  (bind _asbp_game_instance (Utilities|Casting|CastToBP_Game_Instance (Game|GetGameInstance)))
  (Default|PlayDemoLevel _asbp_game_instance))

(event EventTick
  (params (DeltaSeconds :type Float%20%28single-precision%29))
  (Utilities|FlowControl|Sequence
    (:then_0
      (CallFunction|TickNutShadow))
    (:then_1
      (if (AI|Components|NavMovement|IsFalling (Variables|Character|GetCharacterMovement))
        (bind _output_get (Variables|Default|SetFallingCounter (+ (Variables|Default|GetFallingCounter) DeltaSeconds)))
        (Variables|Default|SetIsFallingVoid (>= _output_get (Variables|Default|GetMaxFallingTimer)))
        (else
          (Variables|Default|SetFallingCounter 0.0)
          (Variables|Default|SetIsFallingVoid false))))
    (:then_2
      (CallFunction|HandleEnemiesFocus))
    (:then_3
      (CallFunction|EnergyAcumulation))))

(fn ConstructionScript)

(fn TickNutShadow
  (bind _returnvalue (Transformation|GetActorLocation))
  (bind _returnvalue_2 (Transformation|GetActorLocation))
  (bind _outhit (Collision|LineTraceByChannel _returnvalue (+ _returnvalue "0.000000,0.000000,-5000.000000") "TraceTypeQuery1" false 0 "None"))
  (Rendering|SetVisibility (Variables|Default|GetShadow) (.bBlockingHit (Collision|BreakHitResult _outhit)) false)
  (Transformation|SetWorldLocation (Variables|Default|GetShadow) (Math|Vector|MakeVector (.x _returnvalue_2) (.y _returnvalue_2) (+ (.z (.ImpactPoint (Collision|BreakHitResult _outhit))) 0.5)) true false)
  (Class|WidgetComponent|SetTintColorandOpacity (Variables|Default|GetShadow) (Utilities|Struct|MakeLinearColor 0.0 0.0 0.0 (Math|Float|Clamp(Float) (- 1.0 (Math|Float|NormalizetoRange (.Distance (Collision|BreakHitResult _outhit)) 0.0 5e+02)) 0.0 0.8))))

(fn HandleEnemiesFocus
  (if (Utilities|Array|IsEmpty (Variables|Default|GetActorsFocus))
    (return)
    (elif (Utilities|Array|IsValidIndex (Variables|Default|GetActorsFocus) (Variables|Default|GetFocusIndex))
      (bind _output_get (LocalVariables|SetTargetFocus (Actor|GetComponentbyClass (Utilities|Array|Get(acopy) (Variables|Default|GetActorsFocus) (Variables|Default|GetFocusIndex)) "/Game/Nutbound/Components/Focusable.Focusable_C")))
      (if (== (Variables|Default|GetFocusCompnent) _output_get)
        (return)
        (else
          (if (Utilities|IsValid (Variables|Default|GetFocusCompnent))
            (Variables|/Game/Nutbound/Components/Focusable.Focusable_C|SetIsFocused (Variables|Default|GetFocusCompnent) false))
          (bind _output_get_2 (Variables|Default|SetFocusCompnent (LocalVariables|GetTargetFocus)))
          (Variables|/Game/Nutbound/Components/Focusable.Focusable_C|SetIsFocused _output_get_2 true)))
      (else
        (return)))))

(fn EnergyAcumulation
  (bind _health (Variables|Default|GetHealth))
  (bind _health_2 (Variables|Default|GetHealth))
  (if (> (Math|Vector|VectorLength (Transformation|GetVelocity)) 0.0)
    (Default|PlayerGainEnergy (Variables|Default|GetHealth) (* (Utilities|Time|GetWorldDeltaSeconds) 2.0))
    (else
      (Default|PlayerLoseEnergy (Variables|Default|GetHealth) (* (Utilities|Time|GetWorldDeltaSeconds) 1.0))))
  (Rendering|SetVisibility (Variables|Default|GetEnergyVFX) (> (Variables|/Game/Nutbound/Components/Health.Health_C|GetCurrentEnergy (Variables|Default|GetHealth)) 0.0) true)
  (Transformation|SetRelativeScale3D (Variables|Default|GetEnergyVFX) (* (Class|KismetMathLibrary|VectorOne) (Math|Float|MapRangeClamped (Variables|/Game/Nutbound/Components/Health.Health_C|GetCurrentEnergy _health) 0.0 (Variables|/Game/Nutbound/Components/Health.Health_C|GetMaxEnergy _health) 0.1 4.0)))
  (Rendering|Components|Light|SetIntensity (Variables|Default|GetSpotLight) (Math|Float|MapRangeClamped (Variables|/Game/Nutbound/Components/Health.Health_C|GetCurrentEnergy _health_2) 0.0 (Variables|/Game/Nutbound/Components/Health.Health_C|GetMaxEnergy _health_2) 5e+02 6e+03)))