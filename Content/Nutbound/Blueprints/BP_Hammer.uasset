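; BP_Hammer is a swinging hammer hazard that instantly kills the player nut character if it overlaps them during the downswing.
; A looping 0.01-second timer, rather than Tick, runs UpdateTime, which lerps the Arrow component's pitch between 0 and -90 degrees, with separate down and up durations.
; The Down flag flips at each end of the swing and gates damage, which equals the player's max health.
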(event EventBeginPlay
  (bind _asbp_nut_character (Utilities|Casting|CastToBP_NutCharacter (Game|GetPlayerCharacter 0)))
  (Variables|Default|SetMain%20Character _asbp_nut_character)
  (Variables|Default|SetTimer 0.0)
  (Variables|Default|SetDown true)
  (Utilities|Time|SetTimerbyFunctionName 0 "UpdateTime" 0.01 true))

(event Collision|EventActorBeginOverlap
  (params (OtherActor :type Actor%20Object%20Reference))
  (bind _main_character (Variables|Default|GetMain%20Character))
  (bind _health (Variables|/Game/Nutbound/Blueprints/BP_NutCharacter.BP_NutCharacter_C|GetHealth _main_character))
  (if (== OtherActor _main_character)
    (if (Variables|Default|GetDown)
      (Default|PlayerTakeDamage _health (Variables|/Game/Nutbound/Components/Health.Health_C|GetMaxHealth _health)))))

(event EventTick
  (params (DeltaSeconds :type Float%20%28single-precision%29)))

(fn ConstructionScript)

(fn UpdateTime
  (bind _arrow (Variables|Default|GetArrow))
  (Variables|Default|SetTimer (+ (Variables|Default|GetTimer) 0.01))
  (if (Variables|Default|GetDown)
    (Variables|Default|Setalpha (/ (Variables|Default|GetTimer) (Variables|Default|GetTimeDown)))
    (Transformation|SetRelativeRotation _arrow (Math|Rotator|MakeRotator 0.0 (Math|Float|Lerp 0.0 -9e+01 (Variables|Default|Getalpha)) 0.0) false false)
    (if (>= (Variables|Default|GetTimer) (Variables|Default|GetTimeDown))
      (Variables|Default|SetDown false)
      (Variables|Default|SetTimer 0.0 :!label _label))
    (else
      (Variables|Default|Setalpha (/ (Variables|Default|GetTimer) (Variables|Default|GetTimeUp)))
      (Transformation|SetRelativeRotation _arrow (Math|Rotator|MakeRotator 0.0 (Math|Float|Lerp -9e+01 0.0 (Variables|Default|Getalpha)) 0.0) false false)
      (if (>= (Variables|Default|GetTimer) (Variables|Default|GetTimeUp))
        (Variables|Default|SetDown true)
        (goto _label)))))