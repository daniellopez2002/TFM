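; BP_Grabber is an actor that attacks the player's BP_NutCharacter through a hitbox and has its own Health.
; An AttackHitbox overlap with the player, gated by HasHitPlayer, deals one damage, calls PLayerHit and launches the player away and upward.
; Tick compares State with CurrentState and prints changes for debugging.
; A debug key (M) damages the Grabber itself.
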(event OnComponentBeginOverlap(AttackHitbox)
  (params (OverlappedComponent :type Primitive%20Component%20Object%20Reference) (OtherActor :type Actor%20Object%20Reference) (OtherComp :type Primitive%20Component%20Object%20Reference) (OtherBodyIndex :type Integer) (bFromSweep :type Boolean) (SweepResult :type Hit%20Result%20Structure%20%28by%20ref%29))
  (bind _self self)
  (bind _maincharacter (Variables|Default|GetMainCharacter))
  (if (not (Variables|Default|GetbHasHitPlayer))
    (if (not (== OtherActor _self))
      (if (== OtherActor _maincharacter)
        (Default|PlayerTakeDamage (Variables|/Game/Nutbound/Blueprints/BP_NutCharacter.BP_NutCharacter_C|GetHealth _maincharacter) 1)
        (Class|TFMBossGrabber|PLayerHit)
        (Character|LaunchCharacter _maincharacter (+ (* (Math|Vector|Normalize (- (Transformation|GetActorLocation _maincharacter) (Transformation|GetActorLocation _self))) 3e+02) "0.000000,0.000000,300.000000") false false)))))

(event EventBeginPlay
  (bind _asbp_nut_character (Utilities|Casting|CastToBP_NutCharacter (Game|GetPlayerCharacter 0)))
  (Variables|Default|SetMainCharacter _asbp_nut_character))

(event Collision|EventActorBeginOverlap
  (params (OtherActor :type Actor%20Object%20Reference)))

(event EventTick
  (params (DeltaSeconds :type Float%20%28single-precision%29))
  (bind _currentstate (Variables|Default|GetCurrentState))
  (if (!= (Utilities|Name|EnumtoName (Variables|Default|GetState)) (Utilities|Name|EnumtoName _currentstate))
    (Variables|Default|SetState _currentstate)
    (Development|PrintString (Utilities|String|EnumtoString _currentstate))))

(event Input|KeyboardEvents|DebugKeyM
  (params (Key :type Key%20Structure :default "None") (ActionValue :type Input%20Action%20Value%20Structure))
  (:Pressed
    (Default|TakeDamage (Variables|Default|GetHealth) 1)))

(fn ConstructionScript)