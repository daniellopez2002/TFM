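; BP_CameraController tracks the active camera zone and its camera state for the main character.
; On BeginPlay, given a valid starting zone, it activates that zone and registers itself with the player character and every BP_CameraZone.
; ChangeCameraZone deactivates the previous zone, adopts the new zone's state and prints a debug message, flagging a zone active only when passed the current one again.
; The character's camera transition call is disconnected.
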(event EventBeginPlay
  (if (Utilities|IsValid (Variables|Default|GetCurrentCameraZone))
    (CallFunction|ChangeCameraZone (Variables|Default|GetCurrentCameraZone))
    (Utilities|FlowControl|Sequence
      (:then_0
        (bind _asbp_main_character (Utilities|Casting|CastToBP_MainCharacter (Pawn|GetControlledPawn (Game|GetPlayerController 0))))
        (Variables|/Game/Nutbound/Blueprints/BP_MainCharacter.BP_MainCharacter_C|SetCameraController _asbp_main_character self)
        (Variables|Default|SetAs%20BP%20Main%20Character _asbp_main_character))
      (:then_1
        (bind _outactors (Actor|GetAllActorsOfClass "/Game/Nutbound/Camera/BP_CameraZone.BP_CameraZone_C"))
        (for _array_element _outactors
          (Variables|/Game/Nutbound/Camera/BP_CameraZone.BP_CameraZone_C|SetCameraController _array_element self))))))

(event Collision|EventActorBeginOverlap
  (params (OtherActor :type Actor%20Object%20Reference)))

(event EventTick
  (params (DeltaSeconds :type Float%20%28single-precision%29)))

(fn ConstructionScript)

(fn ChangeCameraZone
  (params (Zone :type BP%20Camera%20Zone%20Object%20Reference))
  (LocalVariables|SetNextCameraZone Zone)
  (if (!= (LocalVariables|GetNextCameraZone) (Variables|Default|GetCurrentCameraZone))
    (if (Utilities|IsValid (Variables|Default|GetCurrentCameraZone))
      (Variables|/Game/Nutbound/Camera/BP_CameraZone.BP_CameraZone_C|SetIsBeenActivated (Variables|Default|GetCurrentCameraZone) false))
    (bind _output_get (Variables|Default|SetCurrentCameraZone (LocalVariables|GetNextCameraZone)))
    (if (Utilities|Enum|Equal(Enum) (Variables|/Game/Nutbound/Camera/BP_CameraZone.BP_CameraZone_C|GetZoneCameraState _output_get) (Variables|Default|GetCameraState))
      _
      (else
        (bind _output_get_2 (Variables|Default|SetCameraState (Variables|/Game/Nutbound/Camera/BP_CameraZone.BP_CameraZone_C|GetZoneCameraState _output_get)))))
    (Development|PrintString (Utilities|String|Append "Change camera zone to:" (Utilities|String|ToString(Object) _output_get) "This zone state is: " (Utilities|String|EnumtoString _output_get_2)) true true "(R=0.094117,G=1.000000,B=0.000000,A=1.000000)")
    (elif (not (Variables|/Game/Nutbound/Camera/BP_CameraZone.BP_CameraZone_C|GetIsBeenActivated (Variables|Default|GetCurrentCameraZone)))
      (Variables|/Game/Nutbound/Camera/BP_CameraZone.BP_CameraZone_C|SetIsBeenActivated (Variables|Default|GetCurrentCameraZone) true))))