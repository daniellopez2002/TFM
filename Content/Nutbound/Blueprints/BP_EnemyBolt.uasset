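; BP_EnemyBolt is an enemy actor in Nutbound with health, a focusable component and a widget component.
; Each tick it sets the widget's visibility from the Focusable component's focus state.
; When the Health component signals death, it hides the mesh and its children, spawns an explosion effect at its location, then destroys itself after a short delay.
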(event OnDeath(Health)
  (Rendering|SetVisibility (Variables|Default|GetMeshComp) false true)
  (Effects|SpawnEmitteratLocation "/Game/StarterContent/Particles/P_Explosion.P_Explosion" (Transformation|GetActorLocation))
  (Utilities|FlowControl|Delay 1.5)
  (Actor|DestroyActor))

(event EventBeginPlay)

(event Collision|EventActorBeginOverlap
  (params (OtherActor :type Actor%20Object%20Reference)))

(event EventTick
  (params (DeltaSeconds :type Float%20%28single-precision%29))
  (Rendering|SetVisibility (Variables|Default|GetWidget) (Variables|/Game/Nutbound/Components/Focusable.Focusable_C|GetIsFocused (Variables|Default|GetFocusable)) false))

(fn ConstructionScript)